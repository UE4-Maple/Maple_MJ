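; BP_MJ_View is a clickable actor that represents a player-owned tile, apparently mahjong, on the game desk.
; A click on its static mesh compares the tile's PlayerID with the ID of the player controller returned by FUNLGetPlayerController.
; On a match it passes itself to the Desk's FUNSelectBoard; otherwise it prints the player's name with a scolding for clicking someone else's tile.
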(event `self.StaticMesh.OnClicked`
  (params (TouchedComponent :type "PrimitiveComponent Object Reference") (ButtonPressed :type "Key Structure"))
  (bind _aspc_main (`/Game/Assets/FUNL_Play.FUNL_GetPlayerController`))
  (if (== (`self.PlayerID`) (`/Game/Assets/PC_Main.ID` _aspc_main))
    (`/Game/Assets/BP/BP_Desk.FUN_Select_Board` (`/Game/Assets/PC_Main.Desk` (`/Game/Assets/FUNL_Play.FUNL_GetPlayerController`)) (`self.PlayerID`) self)
    (else
      (`KismetSystemLibrary.PrintString` (`KismetStringLibrary.Concat_StrStr` (`KismetTextLibrary.Conv_TextToString` (`/Game/Assets/PC_Main.Name` _aspc_main)) "-" "你点别人牌干屌")))))

(fn `UserConstructionScript`
  (`parent.UserConstructionScript`))
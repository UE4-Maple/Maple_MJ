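; BP_Desk is the mahjong table actor: it seats four players, deals and runs draw, discard, pong, kong and win.
; It shuffles the game mode's tiles, deals on timed loops and tracks hands in PlayerInfos, mirrored by per-seat wall, hand and meld components plus a shared discard component.
; NowFetch, NowAlreadyFetch and a post-discard countdown gate actions, with Can functions returning Chinese button text.
; Player controllers relay messages, play-out events and reset.
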(event `self.ReceiveBeginPlay`
  (set `self.Chairs` (`|MakeArray` (`self.Chair1`) (`self.Chair2`) (`self.Chair3`) (`self.Chair4`)))
  (set `self.Views` (`|MakeArray` (`self.Com_View1`) (`self.Com_View2`) (`self.Com_View3`) (`self.Com_View4`)))
  (set `self.Downs` (`|MakeArray` (`self.Com_Down1`) (`self.Com_Down2`) (`self.Com_Down3`) (`self.Com_Down4`)))
  (set `self.Caches` (`|MakeArray` (`self.Com_Cache1`) (`self.Com_Cache2`) (`self.Com_Cache3`) (`self.Com_Cache4`)))
  (bind _output_get (set `self.Widgets` (`|MakeArray` (`self.Widget1`) (`self.Widget2`) (`self.Widget3`) (`self.Widget4`))))
  (for (_array_element _array_index) _output_get
    (bind _asumg_3dtext (cast `/Game/Assets/UMG/UMG_3DText` (`WidgetComponent.GetUserWidgetObject` _array_element) :!pure true))
    (set `/Game/Assets/UMG/UMG_3DText.Desk` self _asumg_3dtext)
    (set `/Game/Assets/UMG/UMG_3DText.Index` _array_index _asumg_3dtext)))

(event `EVE_Start_CD_Fetch`
  (set `self.CD_Fetch` 5)
  (if (> (`self.CD_Fetch`) 0) :!label _label
    (`/Engine/EditorBlueprintResources/StandardMacros.DecrementInt` (`self.CD_Fetch`)
      (:`  `
        (`KismetSystemLibrary.Delay` 1.0)
        (goto _label)))))

(event `EVE_Start`
  (bind _output_get (set `self.All Board` (`/Game/Assets/GM_Main.FUN_GetGroupBoard` (`/Game/Assets/FUNL_Play.FUNL_GetGameMode`))))
  (`KismetArrayLibrary.Array_Shuffle` _output_get)
  (`self.FUN_Down_Init`)
  (`/Game/Assets/PC_Main.EVE_Server_Add_Message` (`/Game/Assets/FUNL_Play.FUNL_GetPlayerController`) "系统：开始发牌")
  (`KismetSystemLibrary.Delay` 2.0)
  (if (<= (`self.L_Index`) 51) :!label _label_2
    (`self.FUN_Down_DestroyOne`)
    (`self.FUN_View_AddOne` (mod (`self.L_Index`) 4))
    (`/Engine/EditorBlueprintResources/StandardMacros.IncrementInt` (`self.L_Index`)
      (:`  `
        (`KismetSystemLibrary.Delay` 0.2)
        (goto _label_2)))
    (else
      (`self.FUN_Set_NowFetch` 0)
      (for _array_element (`self.PlayerInfos`)
        (`/Game/Assets/PC_Main.EVE_Client_ShowCursor` (`.PC_13_F44D405F4B5463726F84EA83F9770246` (break `/Game/Assets/BP/Str_PlayerInfo` _array_element)) true))
      (`/Game/Assets/PC_Main.EVE_Server_Add_Message` (`/Game/Assets/FUNL_Play.FUNL_GetPlayerController`) "系统：发牌完成，请1号抓牌"))))

(fn `FUN_Can_Fetch`
  (params (PlayerID :type Integer))
  (returns (ReturnValue :type Boolean) (Text :type Text))
  (bind _cd_fetch (`self.CD_Fetch`))
  (bind _returnvalue (== _cd_fetch 0))
  (bind _infoindex (`self.FUN_FindPlayer_ByID` PlayerID))
  (if (== _infoindex (`self.Now_Fetch`))
    (if (`self.Now_AlreadyFetch`)
      (return false "已抓")
      (else
        (return _returnvalue (select `bool` _returnvalue :`false` (`|FormatText` "抓牌 {cd} " _cd_fetch) :`true` "抓牌"))))
    (else
      (return false "不可抓"))))

(fn `FUN_Can_Out`
  (params (PlayerID :type Integer) (BoardIndex :type Integer) (Num :type Integer))
  (returns (ReturnValue :type Boolean) (Text :type Text))
  (if (or (== Num 1) (== Num 4))
    (bind _infoindex (`self.FUN_FindPlayer_ByID` (`local.PlayerID`)))
    (if (== _infoindex (`self.Now_Fetch`))
      (if (`self.Now_AlreadyFetch`)
        (return true "出牌")
        (else
          (return false "请 先抓牌")))
      (else
        (return false "非你出")))
    (elif (`self.Now_AlreadyFetch`)
      (return false "下家已抓牌")
      (else
        (bind (_return _boardindex) (`/Game/Assets/BP/Com_Up.FUN_Get_Last` (`self.Com_Up`)))
        (if _return
          (if (== _boardindex (`local.BoardIndex`))
            (return true "碰杠")
            (else
              (return false "碰个屌，你睁大眼睛看看场上什么牌")))
          (else
            (return false "场上没牌，碰你妹碰")))))))

(fn `FUN_Check_BoardEqual`
  (params (View :type "Array of /Game/Assets/BP/BP_MJ_View Object Reference"))
  (returns (ReturnValue :type Boolean) (Index :type Integer))
  (locals (Local :type Integer :default 0))
  (set `local.Local` (`/Game/Assets/BP/BP_MJ.Index` (`|GetArrayItem` View)))
  (for _array_element View
    (if (!= (`/Game/Assets/BP/BP_MJ.Index` _array_element) (`local.Local`))
      (return false 0)))
  (return true (`local.Local`)))

(fn `FUN_Down_DestroyOne`
  (returns (ReturnValue :type Boolean))
  (for _array_element (`self.Downs`)
    (if (> (`KismetArrayLibrary.Array_Length` (`/Game/Assets/BP/Com_Down.All` _array_element)) 0)
      (`/Game/Assets/BP/Com_Down.FUN_DestroyOne` _array_element)
      (return true)))
  (return false))

(fn `FUN_Down_Init`
  (bind _returnvalue (/ (`KismetArrayLibrary.Array_Length` (`self.All Board`)) 4))
  (`/Game/Assets/BP/Com_Down.FUN_SpawnGroupsDown` (`self.Com_Down1`) _returnvalue)
  (`/Game/Assets/BP/Com_Down.FUN_SpawnGroupsDown` (`self.Com_Down2`) _returnvalue)
  (`/Game/Assets/BP/Com_Down.FUN_SpawnGroupsDown` (`self.Com_Down3`) _returnvalue)
  (`/Game/Assets/BP/Com_Down.FUN_SpawnGroupsDown` (`self.Com_Down4`) _returnvalue))

(fn `FUN_Fetch`
  (params (PC :type "/Game/Assets/PC_Main Object Reference"))
  (bind _returnvalue (`self.FUN_Down_DestroyOne`))
  (if _returnvalue
    (`self.FUN_View_AddOne` (`/Game/Assets/PC_Main.ID` PC))
    (set `self.Now_AlreadyFetch` true)
    (`/Game/Assets/PC_Main.EVE_Server_Add_Message` PC (`|FormatText` "{name} 抓牌了" (`/Game/Assets/PC_Main.Name` PC)))
    (else
      (`/Game/Assets/PC_Main.EVE_Server_Add_Message` PC "没有牌了 这把结束了"))))

(fn `FUN_FindPlayer_ByID`
  (params (ID :type Integer))
  (returns (InfoIndex :type Integer))
  (for (_array_element _array_index) (`self.PlayerInfos`)
    (if (== (`.ID_11_BB6776DF413DDDE1AFDB89A62B3616FE` (break `/Game/Assets/BP/Str_PlayerInfo` _array_element)) ID)
      (return _array_index))))

(fn `FUN_Hu`
  (params (PlayerID :type Integer))
  (bind _playerinfos (`self.PlayerInfos`))
  (bind _infoindex (`self.FUN_FindPlayer_ByID` PlayerID))
  (for (_array_element _array_index) (`self.Views`)
    (`/Game/Assets/BP/Com_View.FUN_ShowAllPlayer` _array_element (`|GetArrayItem` _playerinfos _array_index)))
  (bind (_id _playername _pc) (break `/Game/Assets/BP/Str_PlayerInfo` (`|GetArrayItem` _playerinfos _infoindex)))
  (`/Game/Assets/PC_Main.EVE_Server_Add_Message` _pc (`|FormatText` "{name} 胡了   本局结束  所有人牌可见" _playername))
  (`/Game/Assets/PC_Main.EVE_Server_ShowReset` _pc))

(fn `FUN_Out`
  (params (SelectViews :type "Array of /Game/Assets/BP/BP_MJ_View Object Reference") (ID :type Integer))
  (bind _selectviews (`local.SelectViews`))
  (bind _selectviews_2 (`local.SelectViews`))
  (bind _returnvalue (`KismetArrayLibrary.Array_Length` (`local.SelectViews`)))
  (bind _output (`|GetArrayItem` (`local.SelectViews`)))
  (bind _returnvalue_2 (== _returnvalue 2))
  (bind _index (`/Game/Assets/BP/BP_MJ.Index` _output))
  (`self.EVE_Start_CD_Fetch`)
  (if (== (`KismetArrayLibrary.Array_Length` (`local.SelectViews`)) 1)
    (`self.FUN_Set_NowFetch` (+ (`self.Now_Fetch`) 1))
    (bind _infoindex (`self.FUN_FindPlayer_ByID` (`local.ID`)))
    (bind ((`PlayerName_12_41FCD77044EC850D5CBFD2A89B38D930` _playername) (`PC_13_F44D405F4B5463726F84EA83F9770246` _pc) (`Boards_16_92EBA94242EDF4E3D19E7EB7A827BF3F` _boards)) (break `/Game/Assets/BP/Str_PlayerInfo` (`|GetArrayItem` (`self.PlayerInfos`) _infoindex)))
    (bind _output_2 (`|GetArrayItem` (`self.Views`) _infoindex))
    (`KismetArrayLibrary.Array_Remove` _boards (`KismetArrayLibrary.Array_Find` (`/Game/Assets/BP/Com_View.All` _output_2) _output))
    (`/Game/Assets/PC_Main.EVE_Server_Play_OutAN` _pc true "" 0 _index 0)
    (`/Game/Assets/PC_Main.EVE_Server_Add_Message` _pc (`|FormatText` "{name} 出牌了" _playername))
    (`/Game/Assets/BP/Com_Up.FUN_AddOne` (`self.Com_Up`) _index)
    (`/Game/Assets/BP/Com_View.FUN_DestroyOne` _output_2 _output)
    (elif (or _returnvalue_2 (== _returnvalue 3))
      (bind _infoindex_2 (`self.FUN_FindPlayer_ByID` (`local.ID`)))
      (`self.FUN_Set_NowFetch` _infoindex_2 _returnvalue_2)
      (bind (_id _playername_2 _pc_2 _siteindex _boards_2) (break `/Game/Assets/BP/Str_PlayerInfo` (`|GetArrayItem` (`self.PlayerInfos`) _infoindex_2)))
      (`/Game/Assets/PC_Main.EVE_Server_Play_OutAN` _pc_2 true _playername_2 _siteindex (`/Game/Assets/BP/BP_MJ.Index` (`|GetArrayItem` _selectviews_2)) (+ (`KismetArrayLibrary.Array_Length` _selectviews_2) 1))
      (`/Game/Assets/PC_Main.EVE_Server_Play_OutAN` _pc_2 false "" 0 0 0)
      (for _array_element (`local.SelectViews`)
        (bind _output_3 (`|GetArrayItem` (`self.Views`) _infoindex_2))
        (`KismetArrayLibrary.Array_Remove` _boards_2 (`KismetArrayLibrary.Array_Find` (`/Game/Assets/BP/Com_View.All` _output_3) _array_element))
        (bind _output_4 (`|GetArrayItem` (`self.Caches`) _infoindex_2))
        (`/Game/Assets/BP/Com_Cache.FUN_AddOne` _output_4 (`/Game/Assets/BP/BP_MJ.Index` _array_element))
        (`/Game/Assets/BP/Com_View.FUN_DestroyOne` _output_3 _array_element))
      (bind _boardindex (`/Game/Assets/BP/Com_Up.FUN_DestroyOne` (`self.Com_Up`)))
      (`/Game/Assets/BP/Com_Cache.FUN_AddOne` _output_4 _boardindex)
      (`/Game/Assets/PC_Main.EVE_Server_Add_Message` _pc_2 (`|FormatText` "{name}   {info}" _playername_2 (select `bool` _returnvalue_2 :`false` "杠" :`true` "碰" :!type "Text")))
      (elif (== (`KismetArrayLibrary.Array_Length` (`local.SelectViews`)) 4)
        (bind _infoindex_3 (`self.FUN_FindPlayer_ByID` (`local.ID`)))
        (`self.FUN_Set_NowFetch` _infoindex_3)
        (bind (_id_2 _playername_3 _pc_3 _siteindex_2 _boards_3) (break `/Game/Assets/BP/Str_PlayerInfo` (`|GetArrayItem` (`self.PlayerInfos`) _infoindex_3)))
        (`/Game/Assets/PC_Main.EVE_Server_Play_OutAN` _pc_3 true _playername_3 _siteindex_2 (`/Game/Assets/BP/BP_MJ.Index` (`|GetArrayItem` _selectviews)) (`KismetArrayLibrary.Array_Length` _selectviews))
        (for _array_element_2 (`local.SelectViews`)
          (bind _output_5 (`|GetArrayItem` (`self.Views`) _infoindex_3))
          (`KismetArrayLibrary.Array_Remove` _boards_3 (`KismetArrayLibrary.Array_Find` (`/Game/Assets/BP/Com_View.All` _output_5) _array_element_2))
          (`/Game/Assets/BP/Com_Cache.FUN_AddOne` (`|GetArrayItem` (`self.Caches`) _infoindex_3) (`/Game/Assets/BP/BP_MJ.Index` _array_element_2))
          (`/Game/Assets/BP/Com_View.FUN_DestroyOne` _output_5 _array_element_2))
        (`/Game/Assets/PC_Main.EVE_Server_Add_Message` _pc_3 (`|FormatText` "{name}   暗杠" _playername_3))))))

(fn `FUN_Select_Board`
  (params (PlayerID :type Integer) (View :type "/Game/Assets/BP/BP_MJ_View Object Reference"))
  (bind _infoindex (`self.FUN_FindPlayer_ByID` PlayerID))
  (`/Game/Assets/BP/Com_View.FUN_Select_One` (`|GetArrayItem` (`self.Views`) _infoindex) View))

(fn `FUN_Select_Get`
  (params (PlayerID :type Integer))
  (returns (Select :type "Array of /Game/Assets/BP/BP_MJ_View Object Reference"))
  (bind _infoindex (`self.FUN_FindPlayer_ByID` PlayerID))
  (bind _select (`/Game/Assets/BP/Com_View.FUN_Get_Select` (`|GetArrayItem` (`self.Views`) _infoindex)))
  (return _select))

(fn `FUN_Set_NowFetch`
  (params (Now_Fetch :type Integer) (Now_AlreadyFetch :type Boolean))
  (bind _output_get (set `self.Now_Fetch` Now_Fetch))
  (if (>= _output_get 4)
    (set `self.Now_Fetch` 0))
  (set `self.Now_AlreadyFetch` Now_AlreadyFetch))

(fn `FUN_Site`
  (params (Com :type "StaticMeshComponent Object Reference") (PC :type "/Game/Assets/PC_Main Object Reference"))
  (bind _com (`local.Com`))
  (bind _name (`/Game/Assets/PC_Main.Name` PC))
  (bind _returnvalue (`KismetArrayLibrary.Array_Find` (`self.Chairs`) Com))
  (`KismetArrayLibrary.Array_Set` (`self.PlayerInfos`) _returnvalue (make `/Game/Assets/BP/Str_PlayerInfo` (`/Game/Assets/PC_Main.ID` PC) _name PC _returnvalue) true)
  (set `/Game/Assets/PC_Main.Desk` self (`local.PC`))
  (`self.K2_SetActorLocation` (`Controller.K2_GetPawn` (`local.PC`)) (+ (`SceneComponent.K2_GetComponentLocation` _com) (* (`SceneComponent.GetRightVector` _com) 120.0) (0.0 0.0 50.0)) false true)
  (`/Game/Assets/PC_Main.EVE_Server_Add_Message` (`local.PC`) (`|FormatText` "{name}  坐下了" _name))
  (`self.FUN_Site_CheckAll`))

(fn `FUN_Site_Can`
  (params (Com :type "StaticMeshComponent Object Reference"))
  (returns (ReturnValue :type Boolean) (Text :type Text))
  (bind _returnvalue (`KismetArrayLibrary.Array_Find` (`self.Chairs`) Com))
  (if (>= _returnvalue 0)
    (if (`KismetTextLibrary.TextIsEmpty` (`.PlayerName_12_41FCD77044EC850D5CBFD2A89B38D930` (break `/Game/Assets/BP/Str_PlayerInfo` (`|GetArrayItem` (`self.PlayerInfos`) _returnvalue))))
      (return true "坐上")
      (else
        _)))
  (return false ""))

(fn `FUN_Site_CheckAll`
  (locals (Can :type Boolean :default true) (Local :type Integer))
  (for _array_element (`self.PlayerInfos`)
    (if (`KismetTextLibrary.TextIsEmpty` (`.PlayerName_12_41FCD77044EC850D5CBFD2A89B38D930` (break `/Game/Assets/BP/Str_PlayerInfo` _array_element)))
      (set `local.Can` false)
      (else
        (`/Engine/EditorBlueprintResources/StandardMacros.IncrementInt` (`local.Local`)))))
  (if (`local.Can`)
    (`self.EVE_Start`)))

(fn `FUN_Sort`
  (params (PlayerID :type Integer))
  (bind _infoindex (`self.FUN_FindPlayer_ByID` PlayerID))
  (bind _output (`|GetArrayItem` (`self.PlayerInfos`) _infoindex))
  (bind (_id _playername _pc _siteindex _boards) (break `/Game/Assets/BP/Str_PlayerInfo` _output))
  (for (_array_element _array_index) _boards
    (for _index (range _array_index (`KismetArrayLibrary.Array_Length` _boards))
      (if (< _array_element (`|GetArrayItem` _boards _index))
        (`KismetArrayLibrary.Array_Swap` _boards _index _array_index))))
  (`/Game/Assets/BP/Com_View.FUN_SortBoard` (`|GetArrayItem` (`self.Views`) _infoindex) _output))

(fn `FUN_View_AddOne`
  (params (PlayerID :type Integer))
  (bind _output (`|GetArrayItem` (`self.All Board`) (`self.FetchIndex`)))
  (bind _infoindex (`self.FUN_FindPlayer_ByID` PlayerID))
  (bind (_id _playername _pc _siteindex _boards) (break `/Game/Assets/BP/Str_PlayerInfo` (`|GetArrayItem` (`self.PlayerInfos`) _infoindex)))
  (`KismetArrayLibrary.Array_Add` _boards _output)
  (`/Game/Assets/BP/Com_View.FUN_AddOne` (`|GetArrayItem` (`self.Views`) _siteindex) _id _output)
  (`/Engine/EditorBlueprintResources/StandardMacros.IncrementInt` (`self.FetchIndex`)
    (:`  `
      (return))))

(fn `UserConstructionScript`)
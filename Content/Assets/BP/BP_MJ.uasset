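; BP_MJ is a board piece actor, likely a mahjong tile, whose face is chosen by an Index scalar parameter on its mesh materials.
; Events named as multicast set that index or move the actor.
; The client-named event shows the real index only when the local PC_Main controller's ID matches PlayerID, otherwise a fixed placeholder index, hiding the face from other players.
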(event `EVE_Multi_SetBoard`
  (params (Index :type Integer))
  (bind _output_get (set `self.Index` Index))
  (`MeshComponent.SetScalarParameterValueOnMaterials` (`self.StaticMesh`) "Index" (`KismetMathLibrary.Conv_IntToDouble` _output_get)))

(event `EVE_Multi_UpdateLocation`
  (params (Location :type "Vector Structure"))
  (`self.K2_SetActorLocation` Location))

(event `EVE_Client_SetBoard`
  (params (Index :type Integer))
  (bind _output_get (set `self.Index` Index))
  (`MeshComponent.SetScalarParameterValueOnMaterials` (`self.StaticMesh`) "Index" (select `bool` (== (`/Game/Assets/PC_Main.ID` (cast `/Game/Assets/PC_Main` (`GameplayStatics.GetPlayerController` 0) :!pure true)) (`self.PlayerID`)) :`false` 45.0 :`true` (`KismetMathLibrary.Conv_IntToDouble` _output_get))))

(fn `UserConstructionScript`)
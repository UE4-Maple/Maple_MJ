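; Player controller for a multiplayer tile game, apparently mahjong, handling desk seating, player actions and the local play UI.
; The local player creates UMG_Play and line-traces from the camera each tick to show join prompts, with left click taking a seat.
; Sort, fetch, out and Hu events forward to the Desk.
; Server events relay messages and UI updates through the GameMode's PCList, and reset respawns the desk and clears tiles.
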(event `self.ReceiveBeginPlay`
  (if (`self.IsLocalPlayerController`)
    (bind _returnvalue (`|CreateWidget` "/Game/Assets/UMG/UMG_Play.UMG_Play_C" self))
    (`UserWidget.AddToViewport` _returnvalue 0)
    (set `self.UMG_Play` _returnvalue)))

(event `EVE_Server_Add_Message`
  (params (`In Text` :type Text))
  ;[1 1 1] 注释
  (for _array_element (`/Game/Assets/GM_Main.PCList` (`/Game/Assets/FUNL_Play.FUNL_GetGameMode`))
    (`self.EVE_Client_AddMessage` _array_element `In Text`)))

(event `EVE_Client_GetName`
  ;[1 1 1] 注释
  (bind _asgi_main (cast `/Game/Assets/GI_Main` (`GameplayStatics.GetGameInstance`)))
  (`self.EVE_Server_SetName` (`/Game/Assets/GI_Main.Name` _asgi_main)))

(event `self.ReceiveTick`
  (params (DeltaSeconds :type "Float (single-precision)"))
  (`self.FUN_Tick`))

(event `EVE_Client_AddMessage`
  (params (`In Text` :type Text))
  (bind _umg_play (`self.UMG_Play`))
  ;[1 1 1] 注释
  (`/Engine/EditorBlueprintResources/StandardMacros.IsValid` _umg_play
    (:`Is Valid`
      (`/Game/Assets/UMG/UMG_Play.FUN_Add_Message` _umg_play `In Text`))))

(event `EVE_Server_SetName`
  (params (Name :type Text))
  ;[1 1 1] 注释
  (if (not (`KismetTextLibrary.TextIsEmpty` Name))
    (set `self.Name` Name)))

(event `InputAction|MouseLeft`
  (params (Key :type "Key Structure"))
  (:`Pressed`
    (bind (_returnvalue _text _desk _com) (`self.FUN_TraceCanJoin`))
    (if _returnvalue
      (`self.EVE_JoinDesk` _desk _com self))))

(event `EVE_Server_Play_OutAN`
  (params (Add :type Boolean) (PlayerName :type Text) (PlayerIndex :type Integer) (Index :type Integer) (Num :type Integer))
  ;[1 1 1] 注释
  (for _array_element (`/Game/Assets/GM_Main.PCList` (`/Game/Assets/FUNL_Play.FUNL_GetGameMode`))
    (`self.EVE_Client_Play_OutAN` _array_element Add PlayerName PlayerIndex Index Num)))

(event `EVE_JoinDesk`
  (params (Desk :type "/Game/Assets/BP/BP_Desk Object Reference") (Com :type "StaticMeshComponent Object Reference") (PC :type "/Game/Assets/PC_Main Object Reference"))
  (`/Game/Assets/BP/BP_Desk.FUN_Site` Desk Com PC)
  (set `self.AlearSite` true))

(event `EVE_Client_Play_OutAN`
  (params (Add :type Boolean) (PlayerName :type Text) (PlayerIndex :type Integer) (Index :type Integer) (Num :type Integer))
  (bind _umg_play (`self.UMG_Play`))
  ;[1 1 1] 注释
  (`/Engine/EditorBlueprintResources/StandardMacros.IsValid` _umg_play
    (:`Is Valid`
      (`/Game/Assets/UMG/UMG_Play.EVE_Play_OutAN` _umg_play Add PlayerName PlayerIndex Index Num))))

(event `EVE_Client_ShowCursor`
  (params (Show :type Boolean))
  (bind _output_get (set `self.bShowMouseCursor` Show))
  (`/Game/Assets/UMG/UMG_Play.FUN_Show_Optation` (`self.UMG_Play`) (select `bool` _output_get :`false` "Collapsed" :`true` "Visible" :!type "ESlateVisibility Enum")))

(event `Key|C`
  (params (Key :type "Key Structure"))
  (:`Pressed`
    (bind _isa (`/Engine/EditorBlueprintResources/StandardMacros.FlipFlop`)
      (:`A`
        _)
      (:`B`
        _))
    (set `self.bShowMouseCursor` _isa)))

(event `EVE_Server_ShowReset`
  ;[1 1 1] 注释
  (for _array_element (`/Game/Assets/GM_Main.PCList` (`/Game/Assets/FUNL_Play.FUNL_GetGameMode`))
    (`self.EVE_Client_ShowReset` _array_element)))

(event `EVE_Sort`
  (`/Game/Assets/BP/BP_Desk.FUN_Sort` (`self.Desk`) (`self.ID`)))

(event `EVE_Fetch`
  (params (PC :type "/Game/Assets/PC_Main Object Reference"))
  (`/Game/Assets/BP/BP_Desk.FUN_Fetch` (`self.Desk`) PC))

(event `EVE_Client_ShowReset`
  ;[1 1 1] 注释
  (if (`KismetSystemLibrary.IsServer`)
    (`/Game/Assets/UMG/UMG_Play.FUN_Show_Reset` (`self.UMG_Play`) "Visible")))

(event `EVE_Out`
  (params (Views :type "Array of /Game/Assets/BP/BP_MJ_View Object Reference (by ref)"))
  (`/Game/Assets/BP/BP_Desk.FUN_Out` (`self.Desk`) Views (`self.ID`)))

(event `EVE_Server_Reset`
  (bind _desk (`self.Desk`))
  ;[1 1 1] 注释
  (bind _output_get (set `self.Location` (`self.K2_GetActorLocation` _desk)))
  (`self.K2_DestroyActor` _desk)
  (for _array_element (`/Game/Assets/GM_Main.PCList` (`/Game/Assets/FUNL_Play.FUNL_GetGameMode`))
    (set `/Game/Assets/PC_Main.AlearSite` false _array_element)
    (set `/Game/Assets/PC_Main.Desk` null _array_element)
    (`self.EVE_Client_ShowCursor` _array_element false))
  (`|SpawnActorFromClass` "/Game/Assets/BP/BP_Desk.BP_Desk_C" (`KismetMathLibrary.MakeTransform` _output_get (`KismetMathLibrary.MakeRotator` 0.0 0.0 (`KismetMathLibrary.RandomFloatInRange` 0.0 360.0))) "Undefined" "OverrideRootScale" null null)
  (bind _outactors (`GameplayStatics.GetAllActorsOfClass` "/Game/Assets/BP/BP_MJ.BP_MJ_C"))
  (for _array_element_2 _outactors
    (`self.K2_DestroyActor` _array_element_2)))

(event `EVE_Hu`
  (params (PlayerID :type Integer))
  (`/Game/Assets/BP/BP_Desk.FUN_Hu` (`self.Desk`) PlayerID))

(fn `FUN_Tick`
  (if (`self.IsLocalPlayerController`)
    (bind (_returnvalue _text) (`self.FUN_TraceCanJoin`))
    (if _returnvalue
      (`/Game/Assets/UMG/UMG_Play.EVE_ShowJoin` (`self.UMG_Play`) _text))))

(fn `FUN_TraceCanJoin`
  (returns (ReturnValue :type Boolean) (Text :type Text) (Desk :type "/Game/Assets/BP/BP_Desk Object Reference") (Com :type "StaticMeshComponent Object Reference"))
  (bind _playercameramanager (`self.PlayerCameraManager`))
  (bind _returnvalue (`PlayerCameraManager.GetCameraLocation` _playercameramanager))
  (if (not (`self.AlearSite`))
    (bind (_outhit _returnvalue_2) (`KismetSystemLibrary.LineTraceSingle` _returnvalue (+ _returnvalue (* (`self.GetActorForwardVector` _playercameramanager) 500.0)) "TraceTypeQuery1" true (`|MakeArray` (`GameplayStatics.GetPlayerCharacter` 0) :!type "Actor Object Reference")))
    (if _returnvalue_2
      (bind (_bblockinghit _binitialoverlap _time _distance _location _impactpoint _normal _impactnormal _physmat _hitactor _hitcomponent) (`GameplayStatics.BreakHitResult` _outhit))
      (bind _asbp_desk (cast `/Game/Assets/BP/BP_Desk` _hitactor))
      (bind `_as静态网格体组件` (cast `StaticMeshComponent` _hitcomponent))
      (bind (_returnvalue_3 _text) (`/Game/Assets/BP/BP_Desk.FUN_Site_Can` _asbp_desk `_as静态网格体组件`))
      (return _returnvalue_3 _text _asbp_desk `_as静态网格体组件`))))

(fn `UserConstructionScript`)
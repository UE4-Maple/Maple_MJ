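; GM_Main is the game mode that tracks connected PC_Main player controllers and exposes the standard board group.
; On PostLogin it sets the controller's ID from the current list length, adds it to PCList, names it by the new count and calls its EVEClientGetName event.
; On logout it removes the controller without renumbering the others.
; FUN_GetGroupBoard simply returns AllBoardStandard.
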(event `self.K2_PostLogin`
  (params (NewPlayer :type "PlayerController Object Reference"))
  (bind _returnvalue (`KismetArrayLibrary.Array_Length` (`self.PCList`)))
  (bind _aspc_main (cast `/Game/Assets/PC_Main` NewPlayer))
  (set `/Game/Assets/PC_Main.ID` _returnvalue _aspc_main)
  (`KismetArrayLibrary.Array_AddUnique` (`self.PCList`) _aspc_main)
  (set `/Game/Assets/PC_Main.Name` (`KismetTextLibrary.Conv_IntToText` _returnvalue) _aspc_main)
  (`/Game/Assets/PC_Main.EVE_Client_GetName` _aspc_main))

(event `self.K2_OnLogout`
  (params (ExitingController :type "Controller Object Reference"))
  (bind _aspc_main (cast `/Game/Assets/PC_Main` ExitingController))
  (`KismetArrayLibrary.Array_RemoveItem` (`self.PCList`) _aspc_main))

(fn `FUN_GetGroupBoard`
  (returns (AllBoard :type "Array of Integer"))
  (return (`self.AllBoard_Standard`)))

(fn `UserConstructionScript`)